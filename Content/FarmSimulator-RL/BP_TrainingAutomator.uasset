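; Training automator for the farm simulator's RL agents that runs repeated "civilization" iterations, started with L and stopped with S.
; L spawns a training manager, doubles time dilation and loops: destroy agents, fuel and rooms, then respawn rooms from a newly created save object's configs.
; A retriggerable delay paces iterations, with ResetCD meant to postpone teardown during activity.
; IterationFinished jumps straight to the next cycle.
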(event `self.ReceiveBeginPlay`
  (bind _returnvalue (`GameplayStatics.CreateSaveGameObject` "/Game/FarmSimulator/Core/BP_SaveGame.BP_SaveGame_C"))
  (set `self.Save Game` _returnvalue)
  (`self.Init Iteration`))

(event `Key|L`
  (params (Key :type "Key Structure"))
  (:`Released`
    ;[1 0.7969 0] Spawn Training Manager
    (bind _returnvalue (`|SpawnActorFromClass` "/Game/FarmSimulator-RL/Learning/BP_RLTrainingManager.BP_RLTrainingManager_C" (`KismetMathLibrary.MakeTransform` (0.0 0.0 0.0)) "Undefined" "MultiplyWithRoot" null null))
    (set `self.Learning Manager` _returnvalue)
    (set `self.Training` true)
    (`GameplayStatics.SetGlobalTimeDilation` 2.0) ; Set Simulation Rate
    (`self.Kill Iteration` :!label _label)
    (if (`self.Training`)
      (`/Engine/EditorBlueprintResources/StandardMacros.IncrementInt` (`self.Iteration Count`)
        (:`  `
          (`self.Init Iteration`) ; This will be followed by kill iteration later... i promise...?
          (`KismetSystemLibrary.RetriggerableDelay` 5.0)
          (goto _label)))
      (else
        (`KismetSystemLibrary.PrintString` (`KismetStringLibrary.Concat_StrStr` "Training Stopped, " (`KismetStringLibrary.Conv_IntToString` (`self.Iteration Count`)) " civilizations elapsed"))))))

(event `Iteration Finished`
  (goto _label))

(event `Key|S`
  (params (Key :type "Key Structure"))
  (:`Released`
    (set `self.Training` false)))

(event `Reset CD`
  (`KismetSystemLibrary.RetriggerableDelay` 5.0))

(fn `Init Iteration`
  (for _array_element (`/Game/FarmSimulator/Core/BP_SaveGame.Rooms` (`self.Save Game`))
    (bind (_minx _miny _maxx _maxy) (break `/Game/FarmSimulator-RL/Environment/ST_RoomConfig` _array_element))
    (`|SpawnActorFromClass` "/Game/FarmSimulator-RL/Environment/BP_Room.BP_Room_C" (`KismetMathLibrary.MakeTransform` (`KismetMathLibrary.MakeVector` (* (+ _minx _maxx) 50) (* (+ _miny _maxy) 50))) "Undefined" "MultiplyWithRoot" null _array_element null)))

(fn `Kill Iteration`
  (`|ExecutionSequence`
    (:`then_0`
      (bind _outactors (`GameplayStatics.GetAllActorsOfClass` "/Game/FarmSimulator-RL/Agent/BP_Agent_Base.BP_Agent_Base_C"))
      (bind (_arrayindex _arrayelement) (`/Engine/EditorBlueprintResources/StandardMacros.ReverseForEachLoop` _outactors)
        (:`LoopBody`
          (`self.K2_DestroyActor` _arrayelement))))
    (:`then_1`
      (bind _outactors_2 (`GameplayStatics.GetAllActorsOfClass` "/Game/FarmSimulator-RL/Environment/BP_Fuel.BP_Fuel_C"))
      (bind (_arrayindex_2 _arrayelement_2) (`/Engine/EditorBlueprintResources/StandardMacros.ReverseForEachLoop` _outactors_2)
        (:`LoopBody`
          (`self.K2_DestroyActor` _arrayelement_2))))
    (:`then_2`
      (bind _outactors_3 (`GameplayStatics.GetAllActorsOfClass` "/Game/FarmSimulator-RL/Environment/BP_Room.BP_Room_C"))
      (bind (_arrayindex_3 _arrayelement_3) (`/Engine/EditorBlueprintResources/StandardMacros.ReverseForEachLoop` _outactors_3)
        (:`LoopBody`
          (`self.K2_DestroyActor` _arrayelement_3))))
    (:`then_3`
      (`KismetSystemLibrary.PrintString` "Killed all Agents, Fuel, then Rooms."))))

(fn `UserConstructionScript`)