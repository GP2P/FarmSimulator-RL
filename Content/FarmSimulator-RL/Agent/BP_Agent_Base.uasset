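; BP_Agent_Base is an agent actor in the FarmSimulator-RL project that collects fuel pickups and exposes a test score.
; Overlapping a BP_Fuel actor adds its FuelAmount to the agent's Fuel, prints the HumanID and new total, then destroys the pickup.
; GetTestScore returns IntrinsicScore, which this Blueprint does not update.
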(event `self.ReceiveActorBeginOverlap`
  (params (OtherActor :type "Actor Object Reference"))
  (bind _asbp_fuel (cast `/Game/FarmSimulator-RL/Environment/BP_Fuel` OtherActor))
  (`self.Add Fuel` _asbp_fuel))

(fn `Add Fuel`
  (params (Fuel :type "/Game/FarmSimulator-RL/Environment/BP_Fuel Object Reference"))
  (bind _output_get (set `self.Fuel` (+ (`/Game/FarmSimulator-RL/Environment/BP_Fuel.Fuel Amount` Fuel) (`self.Fuel`))))
  (`KismetSystemLibrary.PrintString` (`KismetStringLibrary.Concat_StrStr` "Human: " (`KismetStringLibrary.Conv_IntToString` (`self.Human ID`)) ", Fuel: " (`KismetStringLibrary.Conv_IntToString` _output_get)))
  (`self.K2_DestroyActor` Fuel))

(fn `Get Test Score`
  (returns (`Test Score` :type "Float (double-precision)"))
  (return (`self.Intrinsic Score`)))

(fn `UserConstructionScript`)