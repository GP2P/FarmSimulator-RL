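; Learning Agents trainer Blueprint for reinforcement learning of BP_Agent_Base agents in the FarmSimulator-RL project.
; It registers a conditional "EntropyReward", granted to each agent whose test score reaches a fixed threshold.
; A time-elapsed completion ends each agent's episode after a fixed duration.
; Episode reset is unimplemented, and the entropy and average IS reward helper functions are empty stubs.
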(event `self.SetupRewards`
  (bind _returnvalue (`ConditionalReward.AddConditionalReward` null "EntropyReward"))
  (set `self.ER` _returnvalue))

(event `self.SetRewards`
  (params (AgentIds :type "Array of Integer (by ref)"))
  (for _array_element AgentIds
    (bind _test_score (`/Game/FarmSimulator-RL/Agent/BP_Agent_Base.Get Test Score` (`self.GetAgent` _array_element "/Game/FarmSimulator-RL/Agent/BP_Agent_Base.BP_Agent_Base_C")))
    (`ConditionalReward.SetConditionalReward` (`self.ER`) _array_element (>= _test_score 5.0))))

(event `self.SetupCompletions`
  (bind _returnvalue (`TimeElapsedCompletion.AddTimeElapsedCompletion` null "TimeConstraint"))
  (set `self.TC` _returnvalue))

(event `self.SetCompletions`
  (params (AgentIds :type "Array of Integer (by ref)"))
  (for _array_element AgentIds
    (`TimeElapsedCompletion.SetTimeElapsedCompletion` (`self.TC`) _array_element 10.0)))

(fn `Add Average IS Reward`)

(fn `Add Entropy Reawrd`)